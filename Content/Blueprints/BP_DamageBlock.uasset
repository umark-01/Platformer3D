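; BP_DamageBlock is a hazard block that repeatedly damages a BP_ThirdPersonCharacter while it stays inside the box overlap.
; Overlap starts a delayed countdown, then a fixed amount is subtracted directly from the character's Health.
; A reinfection delay restarts the cycle if the block is still active.
; A BlockState switch recolors the mesh white, orange or red for inactive, active and damaging.
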(event `self.Box.OnComponentBeginOverlap`
  (params (OverlappedComponent :type "PrimitiveComponent Object Reference") (OtherActor :type "Actor Object Reference") (OtherComp :type "PrimitiveComponent Object Reference") (OtherBodyIndex :type Integer) (bFromSweep :type Boolean) (SweepResult :type "HitResult Structure (by ref)"))
  (cast `/Game/ThirdPerson/Blueprints/BP_ThirdPersonCharacter` OtherActor)
  (set `self.bIsActive` true)
  (set `self.BlockState` "NewEnumerator1")
  (`self.StartDamageCountdown`))

(event `self.Box.OnComponentEndOverlap`
  (params (OverlappedComponent :type "PrimitiveComponent Object Reference") (OtherActor :type "Actor Object Reference") (OtherComp :type "PrimitiveComponent Object Reference") (OtherBodyIndex :type Integer))
  (set `self.bIsActive` false)
  (set `self.BlockState` "NewEnumerator0")
  (`self.ChangeBlockColor`))

(event `StartDamageCountdown`
  (`self.ChangeBlockColor`)
  (`KismetSystemLibrary.Delay` (`self.TimeToDamage`))
  (`self.DealDamage`))

(event `DealDamage`
  (if (`self.bIsActive`)
    (set `self.BlockState` "NewEnumerator2")
    (`self.ChangeBlockColor`)
    (bind _asbp_third_person_character (cast `/Game/ThirdPerson/Blueprints/BP_ThirdPersonCharacter` (stale `self.Box.OnComponentBeginOverlap` OtherActor)))
    (set `/Game/ThirdPerson/Blueprints/BP_ThirdPersonCharacter.health` (- (`/Game/ThirdPerson/Blueprints/BP_ThirdPersonCharacter.health` _asbp_third_person_character) 55.0) _asbp_third_person_character)
    (`KismetSystemLibrary.Delay` 0.2)
    (`self.Reinfection Timer`)))

(event `Reinfection Timer`
  (set `self.BlockState` "NewEnumerator0")
  (`self.ChangeBlockColor`)
  (`KismetSystemLibrary.Delay` (`self.ReinfectionDelay`))
  (if (`self.bIsActive`)
    (set `self.BlockState` "NewEnumerator1")
    (`self.StartDamageCountdown`)))

(event `ChangeBlockColor`
  (bind _staticmesh (`self.StaticMesh`))
  (switch `/Game/EBlockState` (`self.BlockState`)
    (:`NewEnumerator0`
      (`PrimitiveComponent.SetMaterial` _staticmesh 0 "/Game/white.white"))
    (:`NewEnumerator1`
      (`PrimitiveComponent.SetMaterial` _staticmesh 0 "/Game/orange.orange"))
    (:`NewEnumerator2`
      (`PrimitiveComponent.SetMaterial` _staticmesh 0 "/Game/red.red"))))

(fn `UserConstructionScript`)