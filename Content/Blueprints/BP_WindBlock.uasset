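; BP_WindBlock is a wind zone actor that pushes the player character sideways along the world Y axis.
; A looping timer periodically randomizes the wind direction to negative, still or positive.
; Box overlap events toggle an in-wind flag and cache the player character, without checking which actor overlapped.
; While the flag is set, Tick offsets the player by wind force and direction, scaled by delta time.
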(event `self.ReceiveBeginPlay`
  (`KismetSystemLibrary.K2_SetTimerDelegate` (delegate `CustomEvent`) 2.0 true))

(event `CustomEvent`
  (set `self.WindDirection` (`KismetMathLibrary.Conv_IntToDouble` (`KismetMathLibrary.RandomIntegerInRange` -1 1))))

(event `self.ReceiveTick`
  (params (DeltaSeconds :type "Float (single-precision)"))
  (if (`self.IsPlayerInWind`)
    (`self.K2_AddActorWorldOffset` (`self.Ref`) (`KismetMathLibrary.MakeVector` 0.0 (* (* DeltaSeconds (`self.WindForce`)) (`self.WindDirection`))) false false)))

(event `self.Box.OnComponentBeginOverlap`
  (params (OverlappedComponent :type "PrimitiveComponent Object Reference") (OtherActor :type "Actor Object Reference") (OtherComp :type "PrimitiveComponent Object Reference") (OtherBodyIndex :type Integer) (bFromSweep :type Boolean) (SweepResult :type "HitResult Structure (by ref)"))
  (bind _asbp_third_person_character (cast `/Game/ThirdPerson/Blueprints/BP_ThirdPersonCharacter` (`GameplayStatics.GetPlayerCharacter` 0)))
  (set `self.Ref` _asbp_third_person_character)
  (set `self.IsPlayerInWind` true))

(event `self.Box.OnComponentEndOverlap`
  (params (OverlappedComponent :type "PrimitiveComponent Object Reference") (OtherActor :type "Actor Object Reference") (OtherComp :type "PrimitiveComponent Object Reference") (OtherBodyIndex :type Integer))
  (set `self.IsPlayerInWind` false))

(fn `UserConstructionScript`)